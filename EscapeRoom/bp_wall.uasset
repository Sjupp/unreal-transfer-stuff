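; Wall actor in the escape room that moves aside while something overlaps its Collider and returns when the overlap ends.
; A timeline lerps the Rube component's relative transform between its starting pose and a configured End location, keeping rotation and scale.
; The CanReachGround flag limits impact effects to the closing move, whose finish spawns a row of P_CustomEffect emitters offset from the root.
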(event OnComponentBeginOverlap(collider)
  (params (OverlappedComponent :type Primitive%20Component%20Object%20Reference) (OtherActor :type Actor%20Object%20Reference) (OtherComp :type Primitive%20Component%20Object%20Reference) (OtherBodyIndex :type Integer) (bFromSweep :type Boolean) (SweepResult :type Hit%20Result%20Structure%20%28by%20ref%29))
  ;[1 1 1] collider overlap events
  (CallFunction|NewTrigger true))

(event OnComponentEndOverlap(collider)
  (params (OverlappedComponent :type Primitive%20Component%20Object%20Reference) (OtherActor :type Actor%20Object%20Reference) (OtherComp :type Primitive%20Component%20Object%20Reference) (OtherBodyIndex :type Integer))
  ;[1 1 1] collider overlap events
  (CallFunction|NewTrigger false))

(event Custom|spawnEmitters
  (bind _defaultsceneroot (Variables|Default|GetDefaultSceneRoot))
  (bind _returnvalue (Transformation|GetRelativeTransform _defaultsceneroot))
  ;[1 1 1] Spawn Emitters on via loop
  (for _index (range -4 4)
    (Effects|SpawnEmitteratLocation "/Game/EscapeRoom/P_CustomEffect.P_CustomEffect" (+ (.location _returnvalue) (Math|Vector|MakeVector -1e+02 (* _index 1.1e+02) 0.0)) (.rotation _returnvalue) (.scale _returnvalue))))

(event Custom|newTrigger
  (params (opening :type Boolean))
  ;[1 1 1] newTrigger
  (if opening
    (Variables|Default|SetcanReachGround false)
    (bind _newtrack_0 (Timeline|Timeline_0 Play)
      (:Update
        (Transformation|SetRelativeTransform (Variables|Default|GetRube) (Math|Transform|Lerp(Transform) (Variables|Default|Getstart) (Variables|Default|Getend) _newtrack_0) false false))
      (:Finished
        (if (stale _output_get)
          (CallFunction|SpawnEmitters))))
    (else
      (bind _output_get (Variables|Default|SetcanReachGround true))
      (Timeline|Timeline_0 Reverse))))

(event EventBeginPlay
  (bind _rube (Variables|Default|GetRube))
  (bind _returnvalue (Transformation|GetRelativeTransform _rube))
  (bind (_location _rotation _scale) (Math|Transform|BreakTransform _returnvalue))
  ;[1 1 1] BeginPlay
  (Variables|Default|Setstart _returnvalue)
  (Variables|Default|Setend (Math|Transform|MakeTransform (.location (Variables|Default|Getend)) _rotation _scale)))

(fn ConstructionScript)