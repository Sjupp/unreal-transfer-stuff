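; Pinball-style flipper actor that swings 45 degrees from its starting rotation, with an enum setting the left or right direction.
; BeginPlay caches the root's relative rotation and computes the active rotation from it.
; The EnterFlipperZone event plays or reverses a timeline based on its boolean, interpolating the root component between the two rotations.
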(event Custom|EnterFlipperZone
  (params (bool :type Boolean))
  (if bool
    (bind _newtrack_0 (Timeline|Timeline_0 Play)
      (:Update
        (Transformation|SetRelativeRotation (Variables|Default|GetDefaultSceneRoot) (Math|Rotator|Lerp(Rotator) (Variables|Default|GetInactiveRotate) (Variables|Default|GetActiveRotate) _newtrack_0) false false)))
    (else
      (Timeline|Timeline_0 Reverse))))

(event EventBeginPlay
  (bind _output_get (Variables|Default|SetInactiveRotate (Variables|/Script/Engine.SceneComponent|GetRelativeRotation (Variables|Default|GetDefaultSceneRoot))))
  (switch Utilities|FlowControl|Switch|SwitchonENUM (Variables|Default|Getenum)
    (:NewEnumerator0
      (Variables|Default|SetActiveRotate (Math|Rotator|CombineRotators _output_get "45.000000,0.000000, 0")))
    (:NewEnumerator1
      (Variables|Default|SetActiveRotate (Math|Rotator|CombineRotators _output_get "-45.000000, 0, 0")))))

(fn ConstructionScript)